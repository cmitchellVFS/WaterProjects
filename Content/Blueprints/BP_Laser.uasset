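; BP_Laser is a laser actor that draws a beam along its forward direction, stopping at the first blocking surface.
; Each Tick it line-traces on the Visibility channel out to VRange and sets the Beam component's BeamEnd vector parameter to the hit location, or to full range when nothing blocks.
; The construction script resets BeamEnd to the actor's location, so the beam starts with zero length.
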(event `self.ReceiveTick`
  (params (DeltaSeconds :type "Float (single-precision)"))
  (bind _returnvalue (`self.K2_GetActorLocation`))
  (bind _returnvalue_2 (+ _returnvalue (* (`self.GetActorForwardVector`) (`self.V_Range`))))
  (set `self.BeamEnd` _returnvalue_2)
  (bind _outhit (`KismetSystemLibrary.LineTraceSingle` _returnvalue _returnvalue_2 "TraceTypeQuery1"))
  (bind (_bblockinghit _binitialoverlap _time _distance _location) (`GameplayStatics.BreakHitResult` _outhit))
  (if _bblockinghit
    (`FXSystemComponent.SetVectorParameter` (`self.Beam`) "BeamEnd" _location)
    (else
      (`FXSystemComponent.SetVectorParameter` (`self.Beam`) "BeamEnd" (`self.BeamEnd`)))))

(fn `UserConstructionScript`
  (bind _output_get (set `self.BeamEnd` (`self.K2_GetActorLocation`)))
  (`FXSystemComponent.SetVectorParameter` (`self.Beam`) "BeamEnd" _output_get))